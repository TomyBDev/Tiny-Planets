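; BP_Number is an actor that displays the current red coin count as a 3D number mesh.
; On BeginPlay it caches a reference to BP_CustomGameState.
; Each Tick it polls the game state's red coin count and, when it changes, swaps its static mesh to the matching numeral from one to eight.
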(event EventTick
  (params (DeltaSeconds :type Float%20%28single-precision%29))
  (bind _gamestateref (Variables|Default|GetGameStateRef))
  (bind _staticmesh (Variables|Default|GetStaticMesh))
  (bind _returnvalue (Class|CustomGameStateBase|GetRedCoins _gamestateref))
  (if (!= _returnvalue (Variables|Default|GetNumber))
    (bind _output_get (Variables|Default|SetNumber _returnvalue))
    (switch int _output_get
      (:1
        (Components|StaticMesh|SetStaticMesh _staticmesh "/Game/Assets/Meshes/Numbers_1.Numbers_1"))
      (:2
        (Components|StaticMesh|SetStaticMesh _staticmesh "/Game/Assets/Meshes/Numbers_2.Numbers_2"))
      (:3
        (Components|StaticMesh|SetStaticMesh _staticmesh "/Game/Assets/Meshes/Numbers_3.Numbers_3"))
      (:4
        (Components|StaticMesh|SetStaticMesh _staticmesh "/Game/Assets/Meshes/Numbers_4.Numbers_4"))
      (:5
        (Components|StaticMesh|SetStaticMesh _staticmesh "/Game/Assets/Meshes/Numbers_5.Numbers_5"))
      (:6
        (Components|StaticMesh|SetStaticMesh _staticmesh "/Game/Assets/Meshes/Numbers_6.Numbers_6"))
      (:7
        (Components|StaticMesh|SetStaticMesh _staticmesh "/Game/Assets/Meshes/Numbers_7.Numbers_7"))
      (:8
        (Components|StaticMesh|SetStaticMesh _staticmesh "/Game/Assets/Meshes/Numbers_8.Numbers_8")))))

(event EventBeginPlay
  (bind _asbp_custom_game_state (Utilities|Casting|CastToBP_CustomGameState (Game|GetGameState)))
  (Variables|Default|SetGameStateRef _asbp_custom_game_state))

(fn ConstructionScript)